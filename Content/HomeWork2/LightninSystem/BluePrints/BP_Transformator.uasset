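; Transformer actor that switches every BPI_Switchable actor, such as lamps, on and off.
; BeginPlay binds an event to the third-person character's E press, and capsule overlap begin and end both call CallInsideCollision for the player's prompt.
; Switch alternates through a FlipFlop, sending on or off interface messages to all switchable actors.
; The Button shift sits inside each loop, so its travel scales with the actor count.
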(event `self.ReceiveBeginPlay`
  ; Подписываемся на событие нажатие кнопки игроком
  (bind _asbp_third_person_character (cast `/Game/HomeWork2/ThirdPerson/Blueprints/BP_ThirdPersonCharacter` (`GameplayStatics.GetPlayerPawn` 0)))
  (add `/Game/HomeWork2/ThirdPerson/Blueprints/BP_ThirdPersonCharacter.Press E` _asbp_third_person_character (`|CreateDelegate` :!event `Switch`)))

(event `self.Capsule.OnComponentBeginOverlap`
  (params (OverlappedComponent :type "PrimitiveComponent Object Reference") (OtherActor :type "Actor Object Reference") (OtherComp :type "PrimitiveComponent Object Reference") (OtherBodyIndex :type Integer) (bFromSweep :type Boolean) (SweepResult :type "HitResult Structure (by ref)"))
  ; Отправляем игроку уведомление о том что он пересек коллизию и нужно вывести текст
  (`self.InsideCollision`))

(event `self.Capsule.OnComponentEndOverlap`
  (params (OverlappedComponent :type "PrimitiveComponent Object Reference") (OtherActor :type "Actor Object Reference") (OtherComp :type "PrimitiveComponent Object Reference") (OtherBodyIndex :type Integer))
  ; Отправляем игроку уведомление о том что он пересек коллизию и нужно вывести текст
  (`self.InsideCollision`))

(event `Switch`
  (bind _button (`self.Button`))
  (bind _button_2 (`self.Button`))
  ; Логика включения и выключения лампочек
  (`/Engine/EditorBlueprintResources/StandardMacros.FlipFlop`
    (:`A`
      (bind _outactors (`GameplayStatics.GetAllActorsWithInterface` "/Game/HomeWork2/LightninSystem/BluePrints/BPI_Switchable.BPI_Switchable_C"))
      (for _array_element _outactors
        (message `/Game/HomeWork2/LightninSystem/BluePrints/BPI_Switchable.SwitchOn` _array_element)
        (`SceneComponent.K2_SetRelativeLocation` _button (+ (`SceneComponent.RelativeLocation` _button) (3.0 0.0 0.0)) false false)))
    (:`B`
      (bind _outactors_2 (`GameplayStatics.GetAllActorsWithInterface` "/Game/HomeWork2/LightninSystem/BluePrints/BPI_Switchable.BPI_Switchable_C"))
      (for _array_element_2 _outactors_2
        (message `/Game/HomeWork2/LightninSystem/BluePrints/BPI_Switchable.SwitchOff` _array_element_2)
        (`SceneComponent.K2_SetRelativeLocation` _button_2 (- (`SceneComponent.RelativeLocation` _button_2) (3.0 0.0 0.0)) false false)))))

(fn `UserConstructionScript`)